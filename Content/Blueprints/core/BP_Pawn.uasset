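; Player pawn for a story-driven heist game, handling per-level startup, inventory and popup UI.
; BeginPlay shows the cursor and switches on level name: Levels 1–3 add their widget and loop shared music by delay, while Levels 0 and 4 show story messages whose button opens Level_1 or MainMenu.
; Inventory edits fire OnUpdateInventory after a short delay.
; Helpers query items and spawn message or image widgets, optionally fullscreen.
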(event `self.ReceiveBeginPlay`
  (set `PlayerController.bShowMouseCursor` true (`GameplayStatics.GetPlayerController` 0))
  (bind _returnvalue (`GameplayStatics.GetCurrentLevelName` true))
  (switch `string` _returnvalue
    (:`Level_1`
      (bind _returnvalue_2 (`|CreateWidget` "/Game/UI/GamePlayWIdgets/WBP_Level_1.WBP_Level_1_C"))
      (`UserWidget.AddToViewport` _returnvalue_2 0)
      (`GameplayStatics.PlaySound2D` "/Game/SFX/S_1.S_1" 1.0 1.0 0.0 null null)
      (bind _returnvalue_3 (`GameplayStatics.SpawnSound2D` "/Game/SFX/S_Level_1.S_Level_1" 1.0 1.0 0.0 null :!label _label))
      (`AudioComponent.Play` _returnvalue_3 0.0)
      (`KismetSystemLibrary.Delay` 138.0)
      (goto _label))
    (:`Level_2`
      (bind _returnvalue_4 (`|CreateWidget` "/Game/UI/GamePlayWIdgets/WBP_Level_2.WBP_Level_2_C"))
      (`UserWidget.AddToViewport` _returnvalue_4 0)
      (goto _label))
    (:`Level_3`
      (bind _returnvalue_5 (`|CreateWidget` "/Game/UI/GamePlayWIdgets/WBP_Level_3.WBP_Level_3_C"))
      (`UserWidget.AddToViewport` _returnvalue_5 0)
      (goto _label))
    (:`Level_0`
      (bind _newparam (message `/Game/Interfaces/BPI_Main.ShowMessage` (`GameplayStatics.GetPlayerPawn` 0) "Под покровом ночи, бесшумно, словно призрак, Виктор проник в дом. Лазерные лучи, сенсоры движения, кодовые замки – ничто не могло остановить профессионала. Но он знал, что настоящая опасность ждет внутри. Профессор Эйнхорн, по слухам, был параноиком и гением, а значит, его дом наверняка полон ловушек и сюрпризов."))
      (add `/Game/UI/Base/WBP_Message.OnClickButton` _newparam (delegate `CustomEvent`)))
    (:`Level_4`
      (bind _newparam_2 (message `/Game/Interfaces/BPI_Main.ShowMessage` (`GameplayStatics.GetPlayerPawn` 0) "Виктор, держа в руках украденную реликвию, уже мысленно делил барыши. Но триумф оказался недолгим. Едва он переступил порог дома, как его оглушили прожекторы, а из темноты вынырнули фигуры в форме, ощетинившиеся оружием. \"Слуги закона\", как он их презрительно называл, ждали его. Кажется, профессор Эйнхорн предвидел его визит и подготовил \"теплый\" прием. Погоня была неизбежна."))
      (add `/Game/UI/Base/WBP_Message.OnClickButton` _newparam_2 (delegate `CustomEvent_1`)))))

(event `CustomEvent`
  (`GameplayStatics.OpenLevel` "Level_1"))

(event `CustomEvent_1`
  (`GameplayStatics.OpenLevel` "MainMenu"))

(event `/Game/Interfaces/BPI_Main.RemoveItem`
  (params (RemoveItem :type Text))
  (bind _items (`self.Items`))
  (for (_array_element _array_index) _items
    (if (`KismetTextLibrary.EqualEqual_TextText` _array_element RemoveItem)
      (`KismetArrayLibrary.Array_Remove` _items _array_index)))
  (`KismetSystemLibrary.Delay` 0.1)
  (`self.OnUpdateInventory`))

(event `/Game/Interfaces/BPI_Main.SetCurrentItem`
  (params (NewItems :type "Array of Text (by ref)"))
  (set `self.Items` NewItems)
  (`KismetSystemLibrary.Delay` 0.1)
  (`self.OnUpdateInventory`))

(event `/Game/Interfaces/BPI_Main.AddItem`
  (params (NewItem :type Text))
  (`KismetArrayLibrary.Array_Add` (`self.Items`) NewItem)
  (`KismetSystemLibrary.Delay` 0.1)
  (`self.OnUpdateInventory`))

(event `/Game/Interfaces/BPI_Main.ShowImage`
  (params (Image :type "Texture2D Object Reference") (FullScreen :type Boolean))
  (if FullScreen
    (bind _returnvalue (`|CreateWidget` "/Game/UI/Base/WBP_ImageFullScreen.WBP_ImageFullScreen_C"))
    (set `/Game/UI/Base/WBP_ImageFullScreen.Image` Image _returnvalue)
    (`UserWidget.AddToViewport` _returnvalue 0)
    (else
      (bind _returnvalue_2 (`|CreateWidget` "/Game/UI/Base/WBP_Image.WBP_Image_C"))
      (set `/Game/UI/Base/WBP_Image.Image` Image _returnvalue_2)
      (`UserWidget.AddToViewport` _returnvalue_2 0))))

(fn `GetCurrentItem`
  (returns (Items :type "Array of Text"))
  (bind _items (`self.Items`))
  (for _ _items
    _)
  (return _items))

(fn `HaveItem`
  (params (Item :type Text))
  (returns (Result :type Boolean))
  (for _array_element (`self.Items`)
    (if (`KismetTextLibrary.EqualEqual_TextText` _array_element (`local.Item`))
      (return true)))
  (return false))

(fn `ShowMessage`
  (params (Message :type Text))
  (returns (NewParam :type "/Game/UI/Base/WBP_Message Object Reference"))
  (bind _returnvalue (`|CreateWidget` "/Game/UI/Base/WBP_Message.WBP_Message_C"))
  (set `/Game/UI/Base/WBP_Message.MessageText` Message _returnvalue)
  (`UserWidget.AddToViewport` _returnvalue 0)
  (return _returnvalue))

(fn `UserConstructionScript`)